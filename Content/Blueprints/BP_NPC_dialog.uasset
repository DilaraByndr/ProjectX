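; NPC dialogue Blueprint that steps through an array of lines shown on screen each time its Talk event fires.
; TalkingToNPC turns off first-person character movement, increments TalkIndex, and writes that Dialogue entry into a WB_Dialogue widget, created once if invalid.
; Past the last line it removes the widget and restores movement; the index is never reset here.
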(event EventTalk
  (CallFunction|TalkingtoNPC))

(fn ConstructionScript)

(fn TalkingtoNPC
  (bind _returnvalue (Actor|GetActorOfClass "/Game/FirstPerson/Blueprints/BP_FirstPersonCharacter.BP_FirstPersonCharacter_C"))
  (Default|CharacterMovementOff _returnvalue)
  (Math|Integer|IncrementInt (Variables|Default|GetTalkIndex)
    (:%20%20
      (if (< (Variables|Default|GetTalkIndex) (Utilities|Array|Length (Variables|Default|GetDialogue)))
        (Variables|Default|GetUI
          (:then
            _)
          (:else
            (bind _returnvalue_2 (UserInterface|CreateWidget "/Game/Dialogues/WB_Dialogue.WB_Dialogue_C" (Game|GetPlayerController 0)))
            (bind _output_get (Variables|Default|SetUI _returnvalue_2))
            (UserInterface|Viewport|AddtoViewport _output_get 0)))
        (Rendering|Components|TextRender|SetText (Variables|/Game/Dialogues/WB_Dialogue.WB_Dialogue_C|GetTalkText (Variables|Default|GetUI)) (Utilities|Text|ToText(String) (Utilities|Array|Get(acopy) (Variables|Default|GetDialogue) (Variables|Default|GetTalkIndex))))
        (else
          (Class|GameViewportSubsystem|RemoveWidget (|GameViewportSubsystem) (Variables|Default|GetUI))
          (bind _returnvalue_3 (Actor|GetActorOfClass "/Game/FirstPerson/Blueprints/BP_FirstPersonCharacter.BP_FirstPersonCharacter_C"))
          (Default|CharacterMovementon _returnvalue_3))))))